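; SMSGameMode_BP is a game mode that runs a countdown in levels and kills the player when time runs out.
; BeginPlay adds a Timer widget and sets the starting minutes and seconds, except in MenuStart.
; Tick uses a Delay to step the countdown once per second while the SMSCharacter is alive, setting its IsDead flag at zero.
; The countdown logic in Tick has no menu-level check.
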(event EventBeginPlay
  (bind _returnvalue (Game|GetCurrentLevelName true))
  (if (not (Utilities|Enum|Equal(Enum) _returnvalue "MenuStart"))
    (bind _returnvalue_2 (UserInterface|CreateWidget "/Game/UI/Timer.Timer_C"))
    (UserInterface|Viewport|AddtoViewport _returnvalue_2 0)
    (Variables|Default|SetTimeMin 3)
    (Variables|Default|SetTimeSec 0)))

(event EventTick
  (params (DeltaSeconds :type Float%20%28single-precision%29))
  (Utilities|FlowControl|Delay 1.0)
  (bind _assmscharacter (Utilities|Casting|CastToSMSCharacter (Game|GetPlayerCharacter 0)))
  (if (not (Variables|/Script/SMS.SMSCharacter|GetbIsDead _assmscharacter))
    (if (<= (Variables|Default|GetTimeSec) 0)
      (if (<= (Variables|Default|GetTimeMin) 0)
        (Variables|/Script/SMS.SMSCharacter|SetbIsDead _assmscharacter true)
        (else
          (Variables|Default|SetTimeMin (- (Variables|Default|GetTimeMin) 1))
          (Variables|Default|SetTimeSec 59)))
      (else
        (Variables|Default|SetTimeSec (- (Variables|Default|GetTimeSec) 1))))))

(fn ConstructionScript)