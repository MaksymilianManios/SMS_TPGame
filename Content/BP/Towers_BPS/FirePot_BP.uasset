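; FirePot_BP is a fire pot actor that explodes and catches fire when the player touches it.
; On overlap with an actor tagged GRACZ, it spawns scaled explosion and fire emitters at its root, along with explosion and spark sounds.
; A WasOverlapedBefore flag, cleared on BeginPlay, makes the effect fire only once, and the fire emitter does not auto-destroy.
; It contains only visual and audio effects, with no damage logic.
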(event EventBeginPlay
  (Variables|Default|SetwasOverlapedBefore false))

(event Collision|EventActorBeginOverlap
  (params (OtherActor :type Actor%20Object%20Reference))
  (bind _defaultsceneroot (Variables|Default|GetDefaultSceneRoot))
  (bind _returnvalue (Transformation|GetWorldLocation _defaultsceneroot))
  (if (not (Variables|Default|GetwasOverlapedBefore))
    (if (Actor|ActorHasTag OtherActor "GRACZ")
      (Effects|SpawnEmitteratLocation "/Game/StarterContent/Particles/P_Explosion.P_Explosion" _returnvalue "0, 0, 0" "10.000000,10.000000,10.000000")
      (Audio|PlaySoundatLocation "/Game/StarterContent/Audio/Explosion01.Explosion01" _returnvalue "0, 0, 0" 1.0 1.0 0.0 0 0 0)
      (Effects|SpawnEmitteratLocation "/Game/StarterContent/Particles/P_Fire.P_Fire" _returnvalue "0, 0, 0" "10.000000,10.000000,10.000000" false)
      (Audio|PlaySoundatLocation "/Game/StarterContent/Audio/Fire_Sparks01_Cue.Fire_Sparks01_Cue" _returnvalue "0, 0, 0" 1.0 1.0 0.0 0 0 0)
      (Variables|Default|SetwasOverlapedBefore true))))

(event EventTick
  (params (DeltaSeconds :type Float%20%28single-precision%29)))

(fn ConstructionScript)