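; Tower emitter actor that keeps a Kula_BP in circulation by spawning one at its Arrow transform on BeginPlay.
; When an actor tagged KULA begins overlapping the Box, it destroys that actor and spawns a fresh Kula_BP at the Arrow.
; Leftover AddImpulseAtLocation nodes are unconnected and never run, so the emitter applies no impulse itself.
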(event OnComponentBeginOverlap(Box)
  (params (OverlappedComponent :type Primitive%20Component%20Object%20Reference) (OtherActor :type Actor%20Object%20Reference) (OtherComp :type Primitive%20Component%20Object%20Reference) (OtherBodyIndex :type Integer) (bFromSweep :type Boolean) (SweepResult :type Hit%20Result%20Structure%20%28by%20ref%29))
  ;[1 1 1] Comment
  (if (Actor|ActorHasTag OtherActor "KULA")
    (Actor|DestroyActor OtherActor)
    (Game|SpawnActorfromClass "/Game/BP/Kula_BP.Kula_BP_C" (Transformation|GetWorldTransform (Variables|Default|GetArrow)) "Undefined" 0 0)))

(event EventBeginPlay
  (Game|SpawnActorfromClass "/Game/BP/Kula_BP.Kula_BP_C" (Transformation|GetWorldTransform (Variables|Default|GetArrow)) "Undefined" 0 0))

(event Collision|EventActorBeginOverlap
  (params (OtherActor :type Actor%20Object%20Reference)))

(event EventTick
  (params (DeltaSeconds :type Float%20%28single-precision%29)))

(fn ConstructionScript)